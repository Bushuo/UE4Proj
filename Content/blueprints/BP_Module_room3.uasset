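; BP_Module_room3 is a room module with helpers for scattering coins, Schlangenkopf and levitate child actors.
; SpawnCoins, SpawnSchlangenkopf and SpawnLevitate each add a child actor at a random point inside their own box component's bounds.
; None of them runs from this Blueprint's events: the coin and Schlangenkopf calls are disconnected, SpawnLevitate has no caller here, and the events and construction script are empty.
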(event `self.ReceiveTick`
  (params (DeltaSeconds :type "Float (single-precision)")))

(event `self.ReceiveBeginPlay`)

(fn `SpawnCoins`
  (bind _coinarea (`self.coinarea`))
  (`AddComponent|ChildActorComponent_3` :`RelativeTransform` (`KismetMathLibrary.Conv_VectorToTransform` (`KismetMathLibrary.RandomPointInBoundingBox` (`SceneComponent.RelativeLocation` _coinarea) (`BoxComponent.BoxExtent` _coinarea)))))

(fn `SpawnLevitate`
  (bind _box (`self.Box`))
  (`AddComponent|ChildActorComponent_1` :`RelativeTransform` (`KismetMathLibrary.Conv_VectorToTransform` (`KismetMathLibrary.RandomPointInBoundingBox` (`SceneComponent.RelativeLocation` _box) (`BoxComponent.BoxExtent` _box)))))

(fn `SpawnSchlangenkopf`
  (bind _schlangenkopfarea (`self.SchlangenkopfArea`))
  (`AddComponent|ChildActorComponent_2` :`RelativeTransform` (`KismetMathLibrary.Conv_VectorToTransform` (`KismetMathLibrary.RandomPointInBoundingBox` (`SceneComponent.RelativeLocation` _schlangenkopfarea) (`BoxComponent.BoxExtent` _schlangenkopfarea)))))

(fn `UserConstructionScript`)